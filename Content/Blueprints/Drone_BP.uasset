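; Drone enemy that roams between six preset locations while spinning at a random yaw rate and shooting at the player.
; FindNextLocation re-calls itself after random delays to pick a new target and spin rate.
; Moving re-arms a short timer, easing the sphere a fixed fraction of the remaining distance each step.
; A BeginPlay delay loop repeatedly aims BulletArrow at the player pawn and spawns Bullet_BP from its transform.
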(event Custom|Moving
  (bind _sphere (Variables|Default|GetSphere))
  (Variables|Default|SetAlpha 0.0)
  (Utilities|Time|SetTimerbyEvent (delegate Custom|Moving) 0.02)
  (Variables|Default|SetAlpha (+ (Variables|Default|GetAlpha) 0.04))
  (Transformation|SetWorldLocation _sphere (Math|Vector|Lerp(Vector) (Transformation|GetWorldLocation _sphere) (Variables|Default|GetLocationToMove) (Variables|Default|GetAlpha)) false false))

(event Custom|FindNextLocation
  (bind _location3 (Variables|Default|GetLocation3))
  (bind _location4 (Variables|Default|GetLocation4))
  (bind _location5 (Variables|Default|GetLocation5))
  (bind _location6 (Variables|Default|GetLocation6))
  (bind _location1 (Variables|Default|GetLocation1))
  (bind _location2 (Variables|Default|GetLocation2))
  (bind _array (Utilities|Array|MakeArray _location1 _location2 _location3 _location4 _location5 _location6))
  (Variables|Default|SetDelta%20Rotation%20Z%20%28Yaw%29 (Math|Random|RandomFloatinRange -5.0 5.0))
  (Variables|Default|SetLocationToMove (Transformation|GetWorldLocation (Utilities|Array|Get(acopy) _array (Math|Random|RandomIntegerinRange 0 (Utilities|Array|LastIndex _array)))))
  (CallFunction|Moving)
  (Utilities|FlowControl|Delay (Math|Random|RandomFloatinRange 1.5 3.0))
  (CallFunction|FindNextLocation))

(event Custom|ShootAtPlayer
  (bind _bulletarrow (Variables|Default|GetBulletArrow))
  ;[1 1 1] This blueprint, takes the arrow that i put on top of the drone and it makes it rotate and look at the player character. It can keep rotating while the drone move arund
  (Transformation|SetWorldRotation _bulletarrow (Math|Rotator|FindLookatRotation (Transformation|GetWorldLocation _bulletarrow) (Transformation|GetWorldLocation (Variables|/Script/Engine.Actor|GetRootComponent (Game|Player|GetPlayerPawn 0)))) false false)
  (Game|SpawnActorfromClass "/Game/Blueprints/Bullet_BP.Bullet_BP_C" (Transformation|GetWorldTransform (Variables|Default|GetBulletArrow)) "Undefined" 0 0))

(event EventBeginPlay
  (CallFunction|FindNextLocation)
  (CallFunction|ShootatPlayer :!label _label)
  (Utilities|FlowControl|Delay 1.75)
  (goto _label))

(event Collision|EventActorBeginOverlap
  (params (OtherActor :type Actor%20Object%20Reference)))

(event EventTick
  (params (DeltaSeconds :type Float%20%28single-precision%29))
  (Transformation|AddLocalRotation (Variables|Default|GetSphere) (Math|Rotator|MakeRotator 0.0 0.0 (Variables|Default|GetDelta%20Rotation%20Z%20%28Yaw%29)) false false))

(fn ConstructionScript)